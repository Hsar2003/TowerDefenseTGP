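; Enemy spawner actor that creates fast enemies (BP_EnemyFast) at its own transform.
; It spawns on BeginPlay, then binds SpawnEnemy to the top-down game mode's RespawnEnemy event for later spawns.
; Each call spawns a single enemy and grows the EnemySpawned and EnemyIncrement counters, but the loop over EnemySpawned has an empty body, so the spawn count stays at one.
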(event Custom|SpawnEnemy
  (Game|SpawnActorfromClass "/Game/Enemy/BP_EnemyFast.BP_EnemyFast_C" (Transformation|GetActorTransform) "AdjustIfPossibleButAlwaysSpawn" "MultiplyWithRoot" 0 0)
  (for _index (range 1 (Variables|Default|GetEnemySpawned))
    _)
  (Math|Integer|IncrementInt (Variables|Default|GetEnemyIncrement)
    (:%20%20
      (Variables|Default|SetEnemySpawned (+ (Variables|Default|GetEnemySpawned) (Variables|Default|GetEnemyIncrement))))))

(event EventBeginPlay
  (CallFunction|SpawnEnemy)
  (bind _asbp_top_down_game_mode (Utilities|Casting|CastToBP_TopDownGameMode (Game|GetGameMode)))
  (EventDispatchers|BindEventtoRespawnEnemy _asbp_top_down_game_mode (delegate Custom|SpawnEnemy)))

(fn ConstructionScript)