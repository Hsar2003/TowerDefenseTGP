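; BP_EnemyFast is an enemy that follows the BP_SplineFast path via a timeline, with rotation fixed to the spline's start.
; It increments the game mode's EnemyAlive on spawn and deals damage to actors overlapping its capsule.
; Incoming damage writes CurrentHealth minus damage into MaxHealth, leaving CurrentHealth unchanged, and destroys the enemy at zero.
; Death leaves EnemyAlive untouched, as the decrement and AIMoveTo-to-goal logic are unconnected.
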(event OnComponentBeginOverlap(CapsuleComponent)
  (params (OverlappedComponent :type Primitive%20Component%20Object%20Reference) (OtherActor :type Actor%20Object%20Reference) (OtherComp :type Primitive%20Component%20Object%20Reference) (OtherBodyIndex :type Integer) (bFromSweep :type Boolean) (SweepResult :type Hit%20Result%20Structure%20%28by%20ref%29))
  (Game|Damage|ApplyDamage OtherActor 5.0 0 0))

(event Custom|MoveAI
  (bind _splineref (Variables|Default|GetSplineRef))
  (Components|Timeline|SetPlayRate (Variables|Default|GetMoving) (/ 2.0 (Variables|Default|GetTimeToCompleteSec)))
  (bind _path1 (Timeline|Moving Play)
    (:Update
      (Transformation|SetActorTransform (Math|Transform|MakeTransform (Spline|GetLocationatDistanceAlongSpline (Variables|/Game/Enemy/BP_SplineFast.BP_SplineFast_C|GetSpline _splineref) (Math|Float|Lerp 0.0 (Spline|GetSplineLength (Variables|/Game/Enemy/BP_SplineFast.BP_SplineFast_C|GetSpline (Variables|Default|GetSplineRef))) _path1) "World") (Spline|GetRotationatDistanceAlongSpline (Variables|/Game/Enemy/BP_SplineFast.BP_SplineFast_C|GetSpline _splineref) 0.0 "Local") "1.000000,1.000000,1.000000")))))

(event EventBeginPlay
  (bind _returnvalue (Actor|GetActorOfClass "/Game/Enemy/BP_SplineFast.BP_SplineFast_C"))
  (Variables|Default|SetSplineRef _returnvalue)
  (bind _asbp_top_down_game_mode (Utilities|Casting|CastToBP_TopDownGameMode (Game|GetGameMode)))
  (Math|Integer|IncrementInt (Variables|/Game/TopDown/Blueprints/BP_TopDownGameMode.BP_TopDownGameMode_C|GetEnemyAlive _asbp_top_down_game_mode)
    (:%20%20
      (CallFunction|MoveAI))))

(event Collision|EventHit
  (params (MyComp :type Primitive%20Component%20Object%20Reference) (Other :type Actor%20Object%20Reference) (OtherComp :type Primitive%20Component%20Object%20Reference) (bSelfMoved :type Boolean) (HitLocation :type Vector :default "0, 0, 0") (HitNormal :type Vector :default "0, 0, 0") (NormalImpulse :type Vector :default "0, 0, 0") (Hit :type Hit%20Result%20Structure%20%28by%20ref%29)))

(event Game|Damage|EventAnyDamage
  (params (Damage :type Float%20%28single-precision%29) (DamageType :type Damage%20Type%20Object%20Reference) (InstigatedBy :type Controller%20Object%20Reference) (DamageCauser :type Actor%20Object%20Reference))
  (if (not (Variables|Default|GetisDead?))
    (bind _output_get (Variables|Default|SetMaxHealth (Math|Float|Clamp(Float) (- (Variables|Default|GetCurrentHealth) Damage) 0.0 5e+01)))
    (Development|PrintString (Utilities|String|ToString(Float) _output_get))
    (if (== _output_get 0.0)
      (Variables|Default|SetisDead? true)
      (Development|PrintString "target is destroyed")
      (Actor|DestroyActor))))

(fn ConstructionScript)