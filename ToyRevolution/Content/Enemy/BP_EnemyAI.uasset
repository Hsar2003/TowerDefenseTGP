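; BP_EnemyAI is an enemy whose mesh follows its own spline and which dies on contact with the player character.
; Tick advances the distance along the spline by a speed variable and moves the mesh to that local location and rotation, with no looping or clamping.
; A hit from BP_TopDownCharacter decrements the game mode's alive-enemy count, calls its remaining-enemy check, then destroys the actor.
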(event EventBeginPlay)

(event EventTick
  (params (DeltaSeconds :type Float%20%28single-precision%29))
  (Variables|Default|SetDistanceAlongSpline (+ (* DeltaSeconds (Variables|Default|GetSplineSpeed)) (Variables|Default|GetDistanceAlongSpline)))
  (Transformation|SetRelativeTransform (Variables|Character|GetMesh) (Math|Transform|MakeTransform (.location (Spline|GetTransformatDistanceAlongSpline (Variables|Default|GetSpline) (Variables|Default|GetDistanceAlongSpline) "Local" false)) (.rotation (Spline|GetTransformatDistanceAlongSpline (Variables|Default|GetSpline) (Variables|Default|GetDistanceAlongSpline) "Local" false)) (Variables|/Script/Engine.SceneComponent|GetRelativeScale3D (Variables|Character|GetMesh))) false false))

(event Collision|EventHit
  (params (MyComp :type Primitive%20Component%20Object%20Reference) (Other :type Actor%20Object%20Reference) (OtherComp :type Primitive%20Component%20Object%20Reference) (bSelfMoved :type Boolean) (HitLocation :type Vector :default "0, 0, 0") (HitNormal :type Vector :default "0, 0, 0") (NormalImpulse :type Vector :default "0, 0, 0") (Hit :type Hit%20Result%20Structure%20%28by%20ref%29))
  (Utilities|Casting|CastToBP_TopDownCharacter Other)
  (bind _asbp_top_down_game_mode (Utilities|Casting|CastToBP_TopDownGameMode (Game|GetGameMode)))
  (Math|Integer|DecrementInt (Variables|/Game/TopDown/Blueprints/BP_TopDownGameMode.BP_TopDownGameMode_C|GetEnemyAlive _asbp_top_down_game_mode)
    (:%20%20
      (Default|CheckEnemyLeft _asbp_top_down_game_mode)
      (Actor|DestroyActor))))

(fn ConstructionScript)