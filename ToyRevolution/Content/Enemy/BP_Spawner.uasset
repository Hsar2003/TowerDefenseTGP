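; BP_Spawner is an enemy spawner actor that produces escalating batches of BP_EnemyAI at its own transform.
; On BeginPlay it binds SpawnEnemy to the respawn-enemy event of BP_TopDownGameMode.
; Each trigger spawns EnemySpawned enemies, ignoring collision, then raises EnemyIncrement by one and adds it to EnemySpawned, so successive batches grow at an accelerating rate.
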(event Custom|SpawnEnemy
  (for _index (range 1 (Variables|Default|GetEnemySpawned))
    (Game|SpawnActorfromClass "/Game/Enemy/BP_EnemyAI.BP_EnemyAI_C" (Transformation|GetActorTransform) "AlwaysSpawn" "MultiplyWithRoot" 0 0))
  (Math|Integer|IncrementInt (Variables|Default|GetEnemyIncrement)
    (:%20%20
      (Variables|Default|SetEnemySpawned (+ (Variables|Default|GetEnemySpawned) (Variables|Default|GetEnemyIncrement))))))

(event EventBeginPlay
  (bind _asbp_top_down_game_mode (Utilities|Casting|CastToBP_TopDownGameMode (Game|GetGameMode)))
  (EventDispatchers|BindEventtoRespawnEnemy _asbp_top_down_game_mode (delegate Custom|SpawnEnemy)))

(fn ConstructionScript)