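; BP_Gate is a damageable gate actor whose destruction ends the game.
; AnyDamage subtracts from a clamped health value and prints it, ignoring hits once the gate is dead.
; At zero health it prints "Game Over", destroys itself, then disables player input and shows the BP_Restart widget.
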(event EventBeginPlay)

(event Collision|EventActorBeginOverlap
  (params (OtherActor :type Actor%20Object%20Reference)))

(event EventTick
  (params (DeltaSeconds :type Float%20%28single-precision%29)))

(event Game|Damage|EventAnyDamage
  (params (Damage :type Float%20%28single-precision%29) (DamageType :type Damage%20Type%20Object%20Reference) (InstigatedBy :type Controller%20Object%20Reference) (DamageCauser :type Actor%20Object%20Reference))
  (bind _returnvalue (Game|GetPlayerController 0))
  (if (not (Variables|Default|GetisDead?))
    (bind _output_get (Variables|Default|SetCurrentHealth (Math|Float|Clamp(Float) (- (Variables|Default|GetCurrentHealth) Damage) 0.0 5e+01)))
    (Development|PrintString (Utilities|String|ToString(Float) _output_get))
    (if (== _output_get 0.0)
      (Variables|Default|SetisDead? true)
      (Development|PrintString "Game Over")
      (Actor|DestroyActor)
      (Input|DisableInput _returnvalue _returnvalue)
      (Utilities|Casting|CastToPlayerController _returnvalue)
      (bind _returnvalue_2 (UserInterface|CreateWidget "/Game/Widget/BP_Restart.BP_Restart_C"))
      (UserInterface|Viewport|AddtoViewport _returnvalue_2 0))))

(fn ConstructionScript)